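; BP_Game is a shared helper Blueprint for level selection, level travel and switching input between UI and gameplay.
; SelectLevel stores and prints a chosen level name, which GoToSelectedLevel later opens, while OpenLevel loads a named level directly.
; SetInputMode toggles UI-only or game-only input along with cursor visibility.
; EndLevelSelect finds the BP_LevelSelectTerminal actor in the world and ends its selection.
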(event `OpenLevel`
  (params (LevelName :type Name))
  (`GameplayStatics.OpenLevel` LevelName))

(event `GoToSelectedLevel`
  (`GameplayStatics.OpenLevel` (`self.SelectedLevel`)))

(event `SelectLevel`
  (params (SelectedLevel :type Name))
  (bind _output_get (set `self.SelectedLevel` SelectedLevel))
  (`KismetSystemLibrary.PrintString` (`KismetStringLibrary.Conv_NameToString` _output_get)))

(event `SetInputMode`
  (params (`IsUI?` :type Boolean))
  (bind _returnvalue (`GameplayStatics.GetPlayerController` 0))
  (bind _returnvalue_2 (`GameplayStatics.GetPlayerController` 0))
  (if `IsUI?`
    (`WidgetBlueprintLibrary.SetInputMode_UIOnlyEx` _returnvalue_2 null)
    (set `PlayerController.bShowMouseCursor` true _returnvalue_2)
    (else
      (`WidgetBlueprintLibrary.SetInputMode_GameOnly` _returnvalue)
      (set `PlayerController.bShowMouseCursor` false _returnvalue))))

(event `EndLevelSelect`
  (bind _returnvalue (`GameplayStatics.GetActorOfClass` "/Game/Blueprints/BP_Mohamed/BP_LevelSelectTerminal.BP_LevelSelectTerminal_C"))
  (`/Game/Blueprints/BP_Mohamed/BP_LevelSelectTerminal.EndSelection` _returnvalue))