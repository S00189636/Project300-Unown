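; Enemy actor that attacks a given target by firing projectiles at it.
; BeginPlay fills health by passing negative MaxHealth to SubtractHealth.
; Attack spawns a BP_Projectile with fixed damage at the enemy's location, rotated toward the target by a look-at helper.
; A ready flag and a delay limit firing to the attack rate.
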(event `self.ReceiveBeginPlay`
  (`parent.ReceiveBeginPlay`)
  (`self.SubtractHealth` (* -1 (`self.MaxHealth`))))

(event `self.Attack`
  (params (TargetActor :type "Actor Object Reference"))
  (if (`self.RedyToAttack`)
    (`|SpawnActorFromClass` "/Game/Blueprints/BP_Simran/BP_Projectile.BP_Projectile_C" (`self.GetTransformAndDiraction` TargetActor) "Undefined" "OverrideRootScale" null 10.0 null)
    (set `self.RedyToAttack` false)
    (`KismetSystemLibrary.Delay` (`self.AttackRate`))
    (set `self.RedyToAttack` true)))

(fn `GetTransformAndDiraction`
  (params (self2 :type "Actor Object Reference"))
  (returns (Transform :type "Transform Structure") (Diraction :type "Vector Structure"))
  (bind _returnvalue (`KismetMathLibrary.FindLookAtRotation` (`self.K2_GetActorLocation`) (`self.K2_GetActorLocation` self2)))
  (return (`KismetMathLibrary.MakeTransform` (`self.K2_GetActorLocation`) _returnvalue) (`KismetMathLibrary.Normal` (`KismetMathLibrary.GetForwardVector` _returnvalue))))

(fn `UserConstructionScript`
  (`parent.UserConstructionScript`))