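; AI controller for a drone enemy that runs the BT_AttackingEnemy behavior tree on BeginPlay.
; Perception updates write directly to the State enum on the controlled BP_EnemyBase pawn.
; A successful sense sets one state, while a failed sense, or any update while the pawn is in a particular excluded state, sets another.
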(event `self.ReceiveBeginPlay`
  (`self.RunBehaviorTree` "/Game/Blueprints/BP_Mohamed/AI_Object/BT_AttackingEnemy.BT_AttackingEnemy"))

(event `self.AIPerception.OnTargetPerceptionUpdated`
  (params (Actor :type "Actor Object Reference") (Stimulus :type "AIStimulus Structure"))
  (bind _asbp_enemy_base (cast `/Game/Blueprints/BP_Mohamed/AI_Object/BP_EnemyBase` (`self.K2_GetPawn`)))
  (if (and (not (`|EnumEquality` (`/Game/Blueprints/BP_Mohamed/AI_Object/BP_EnemyBase.State` _asbp_enemy_base) "NewEnumerator5")) (`.bSuccessfullySensed` (break `AIStimulus` Stimulus)))
    (set `/Game/Blueprints/BP_Mohamed/AI_Object/BP_EnemyBase.State` "NewEnumerator1" _asbp_enemy_base)
    (else
      (set `/Game/Blueprints/BP_Mohamed/AI_Object/BP_EnemyBase.State` "NewEnumerator6" _asbp_enemy_base))))

(fn `UserConstructionScript`)