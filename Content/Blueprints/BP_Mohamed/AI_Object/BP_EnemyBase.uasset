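; BP_EnemyBase is a base enemy character with state tracking, look-at rotation, type-filtered damage and levitation hooks.
; TakeDamage subtracts health only for the matching damage type, calling Die when depleted.
; Die sets the death state, ragdolls the mesh and removes the capsule.
; StartLevitate just returns the mesh, EndLevitate restores its gravity, and Attack is a placeholder that toggles readiness and prints.
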(event `self.ReceiveBeginPlay`
  (`parent.ReceiveBeginPlay`)
  (set `self.ReturnComp` (`self.Mesh`)))

(fn `Attack`
  (params (TargetActor :type "Actor Object Reference"))
  (if (`self.RedyToAttack`)
    (`KismetSystemLibrary.PrintString` "Enemy Attacking")
    (set `self.RedyToAttack` false)
    (else
      (set `self.RedyToAttack` true))))

(fn `Die`
  (if (not (`|EnumEquality` (`self.State`) "NewEnumerator5"))
    (`self.SetState` "NewEnumerator5")
    (`PrimitiveComponent.SetSimulatePhysics` (`self.ReturnComp`) true)
    (`ActorComponent.K2_DestroyComponent` (`self.CapsuleComponent`))
    (`PrimitiveComponent.SetCollisionResponseToChannel` (`self.ReturnComp`) "ECC_Visibility" "ECR_Block")))

(fn `EndLevitate`
  (returns (Ended :type Boolean))
  (`PrimitiveComponent.SetEnableGravity` (`self.Mesh`) true)
  (return false))

(fn `LookAtActor`
  (params (OtherActor :type "Actor Object Reference"))
  (`self.K2_SetActorRotation` (`KismetMathLibrary.FindLookAtRotation` (`self.K2_GetActorLocation`) (`self.K2_GetActorLocation` OtherActor))))

(fn `SetState`
  (params (State :type "/Game/Blueprints/BP_Mohamed/AI_Object/E_EnemyState Enum" :default "NewEnumerator0"))
  (set `self.PreviousState` (`self.State`))
  (set `self.State` State))

(fn `StartLevitate`
  (params (Power :type "Float (double-precision)") (Direction :type "Vector Structure"))
  (returns (outComp :type "PrimitiveComponent Object Reference"))
  (return (`self.ReturnComp`)))

(fn `TakeDamage`
  (params (DamageType :type "/Game/Blueprints/BP_Mohamed/E_DamageType Enum" :default "NewEnumerator0") (Amount :type "Float (double-precision)"))
  (returns (Dead :type Boolean))
  (if (`|EnumInequality` (`self.State`) "NewEnumerator5")
    (if (`|EnumEquality` DamageType (`self.TakeDamageFromType`))
      (bind _returnvalue (`self.SubtractHealth` Amount))
      (if _returnvalue
        (`self.Die`)
        (return true))
      (else
        (`KismetSystemLibrary.PrintString` "This dose not work on me ")
        (return false)))
    (else
      (return true))))

(fn `UserConstructionScript`)