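; A fire damage box that deals periodic damage to the player while they stand inside its DamageArea volume.
; BeginPlay creates a looping damage timer and immediately pauses it.
; Overlap by the player character caches its MainPlayerState and unpauses the timer, which calls TakeDamageToHealth on that state, and end overlap pauses it again.
; Only the most recently entered player's state is stored and damaged.
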(event `self.ReceiveBeginPlay`
  (bind _returnvalue (`KismetSystemLibrary.K2_SetTimerDelegate` (delegate `DealDamageToActor`) (`self.DelayDuration`) true))
  (bind _output_get (set `self.DamageTimerHandle` _returnvalue))
  (`KismetSystemLibrary.K2_PauseTimerHandle` _output_get))

(event `DealDamageToActor`
  (`MainPlayerState.TakeDamageToHealth` (`self.As Main Player State`) (`self.DamageAmount`)))

(event `self.DamageArea.OnComponentBeginOverlap`
  (params (OverlappedComponent :type "PrimitiveComponent Object Reference") (OtherActor :type "Actor Object Reference") (OtherComp :type "PrimitiveComponent Object Reference") (OtherBodyIndex :type Integer) (bFromSweep :type Boolean) (SweepResult :type "HitResult Structure (by ref)"))
  (bind _asmy_player_character (cast `MyPlayerCharacter` OtherActor))
  (bind _asmain_player_state (cast `MainPlayerState` (`Pawn.PlayerState` _asmy_player_character)))
  (set `self.As Main Player State` _asmain_player_state)
  (`KismetSystemLibrary.K2_UnPauseTimerHandle` (`self.DamageTimerHandle`)))

(event `self.DamageArea.OnComponentEndOverlap`
  (params (OverlappedComponent :type "PrimitiveComponent Object Reference") (OtherActor :type "Actor Object Reference") (OtherComp :type "PrimitiveComponent Object Reference") (OtherBodyIndex :type Integer))
  (cast `MyPlayerCharacter` OtherActor)
  (`KismetSystemLibrary.K2_PauseTimerHandle` (`self.DamageTimerHandle`)))

(fn `UserConstructionScript`)