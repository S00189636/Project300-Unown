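; An interactable level select terminal that shows a selection screen and controls the visibility of a linked Portal actor, which starts hidden.
; Interact needs no key; it shows the Screen, switches input mode and hides the HUD through BP_Game, and blends the camera to the terminal.
; EndSelection hides the Screen, blends the view back to the player and reveals the Portal if BP_Game has a SelectedLevel.
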(event `self.ReceiveBeginPlay`
  (`self.SetActorHiddenInGame` (`self.Portal`) true))

(fn `EndSelection`
  (bind _asbp_game (cast `/Game/Blueprints/Main_BP_SharedFolder/BP_Game` (`GameplayStatics.GetGameInstance`)))
  (if (!= (`/Game/Blueprints/Main_BP_SharedFolder/BP_Game.SelectedLevel` _asbp_game) "None")
    (`self.SetActorHiddenInGame` (`self.Portal`) false))
  (`SceneComponent.SetHiddenInGame` (`self.Screen`) true true)
  (`PlayerController.SetViewTargetWithBlend` (`GameplayStatics.GetPlayerController` 0) (`GameplayStatics.GetPlayerCharacter` 0) 0.5 "VTBlend_Linear" 0.0 true))

(fn `GetKey`
  (returns (Key :type Name) (Needkey :type Boolean))
  (return "None" false))

(fn `Interact`
  (returns (`Success ` :type Boolean))
  (`SceneComponent.SetHiddenInGame` (`self.Screen`) false true)
  (bind _asbp_game (cast `/Game/Blueprints/Main_BP_SharedFolder/BP_Game` (`GameplayStatics.GetGameInstance`)))
  (`/Game/Blueprints/Main_BP_SharedFolder/BP_Game.SetInputMode` _asbp_game true)
  (`PlayerController.SetViewTargetWithBlend` (`GameplayStatics.GetPlayerController` 0) self 1.0 "VTBlend_Linear" 0.0 true)
  (bind _asbp_game_2 (cast `/Game/Blueprints/Main_BP_SharedFolder/BP_Game` (`GameplayStatics.GetGameInstance`)))
  (`/Game/Blueprints/Main_BP_SharedFolder/BP_Game.HidePlayerHUD` _asbp_game_2)
  (return true))

(fn `UserConstructionScript`)