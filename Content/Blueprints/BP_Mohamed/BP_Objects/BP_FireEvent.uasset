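; BP_FireEvent is an overlap-triggered scripted event that starts when MyPlayerCharacter enters it.
; It plays a 2D sound, waits briefly, destroys the ObjectsDelete actors, enables physics on Objects meshes and shows the ParticleSystems emitters.
; The particle reveal and IsTriggered guard are set inside the Objects loop, so both repeat per object, require a non-empty array, and leave the event re-triggerable during the delay.
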(event `self.ReceiveActorBeginOverlap`
  (params (OtherActor :type "Actor Object Reference"))
  (if (not (`self.IsTriggered`))
    (cast `MyPlayerCharacter` OtherActor)
    (`GameplayStatics.PlaySound2D` (`self.Sound`) 1.0 1.0 0.5 null null)
    (`KismetSystemLibrary.Delay` 0.2)
    (for _array_element (`self.Objects_Delete`)
      (`self.K2_DestroyActor` _array_element))
    (for _array_element_2 (`self.Objects`)
      (`PrimitiveComponent.SetSimulatePhysics` (`StaticMeshActor.StaticMeshComponent` _array_element_2) true)
      (for _array_element_3 (`self.Particle Systems`)
        (`SceneComponent.SetVisibility` (`Emitter.ParticleSystemComponent` _array_element_3) true false))
      (set `self.IsTriggered` true))))

(fn `UserConstructionScript`
  (`parent.UserConstructionScript`))