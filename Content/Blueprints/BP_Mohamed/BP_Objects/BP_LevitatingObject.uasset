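; BP_LevitatingObject is an object that can be levitated and shows a glow aura on its static mesh while levitating.
; StartLevitate turns the aura on and returns the mesh to the caller, while EndLevitate turns it off and returns false.
; ToggleAura caches slot 0's material as a dynamic instance, swaps in a floating-glow instance with its aura parameter enabled, then restores the cached material when switched off.
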(fn `EndLevitate`
  (returns (Ended :type Boolean))
  (`self.ToggleAura` 0)
  (return false))

(fn `StartLevitate`
  (returns (outComp :type "PrimitiveComponent Object Reference"))
  (`self.ToggleAura` 1)
  (return (`self.StaticMesh`)))

(fn `ToggleAura`
  (params (isOn :type Integer))
  (bind _staticmesh (`self.StaticMesh`))
  (if (> isOn 0)
    (bind _returnvalue (`PrimitiveComponent.CreateDynamicMaterialInstance` _staticmesh 0 (`|GetArrayItem` (`MeshComponent.GetMaterials` _staticmesh)) "None"))
    (set `self.OriginalMaterial` _returnvalue)
    (bind _returnvalue_2 (`PrimitiveComponent.CreateDynamicMaterialInstance` _staticmesh 0 "/Game/Materials/M_Mohamed/M_FloatingGlow_Inst.M_FloatingGlow_Inst" "None"))
    (`MaterialInstanceDynamic.SetScalarParameterValue` _returnvalue_2 "IsAuraOn" (`KismetMathLibrary.Conv_IntToDouble` 1))
    (else
      (`PrimitiveComponent.CreateDynamicMaterialInstance` (`self.StaticMesh`) 0 (`self.OriginalMaterial`) "None"))))

(fn `UserConstructionScript`)