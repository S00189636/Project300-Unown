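; BP_PathNode is a placeable path node actor that links to another node through its Next reference.
; Its Construction Script rotates an Arrow component to point from this node toward Next, showing the link direction.
; When Next is not valid, it hides the arrow.
; The event graph holds only disabled stub events, so the node has no runtime logic of its own.
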(fn `UserConstructionScript`
  (`/Engine/EditorBlueprintResources/StandardMacros.IsValid` (`self.Next`)
    (:`Is Valid`
      (`SceneComponent.K2_SetWorldRotation` (`self.Arrow`) (`KismetMathLibrary.FindLookAtRotation` (`SceneComponent.K2_GetComponentLocation` (`self.DefaultSceneRoot`)) (`SceneComponent.K2_GetComponentLocation` (`Actor.RootComponent` (`self.Next`)))) false false))
    (:`Is Not Valid`
      (`SceneComponent.SetVisibility` (`self.Arrow`) false false))))