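; BP_EventTrigger is a one-shot trigger actor that fires a scripted physics event when the player character overlaps it.
; On overlap it plays a 2D sound, waits briefly, destroys the actors in ObjectsDelete, then enables physics simulation on the static meshes in Objects.
; IsTriggered is only set inside that final loop, after the delay, so it stays unset if Objects is empty.
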(event `self.ReceiveActorBeginOverlap`
  (params (OtherActor :type "Actor Object Reference"))
  (if (not (`self.IsTriggered`))
    (cast `/Game/Blueprints/BP_Mohamed/Player/BP_PlayerCharecter_Moh` OtherActor)
    (`GameplayStatics.PlaySound2D` (`self.Sound`) 1.0 1.0 0.5 null null)
    (`KismetSystemLibrary.Delay` 0.2)
    (for _array_element (`self.Objects_Delete`)
      (`self.K2_DestroyActor` _array_element))
    (for _array_element_2 (`self.Objects`)
      (`PrimitiveComponent.SetSimulatePhysics` (`StaticMeshActor.StaticMeshComponent` _array_element_2) true)
      (set `self.IsTriggered` true))))

(fn `UserConstructionScript`)