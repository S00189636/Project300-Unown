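; BP_ShowMessageTrigger is a trigger actor that repeatedly shows a tooltip message while the player character is inside it.
; BeginPlay creates a looping timer that calls ShowToolTip with MessageText every Duration seconds, then immediately pauses it.
; Player overlap unpauses the timer and leaving pauses it.
; The first message therefore waits for the timer to elapse, and progress carries across visits.
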(event `self.ReceiveBeginPlay`
  (bind _returnvalue (`KismetSystemLibrary.K2_SetTimerDelegate` (delegate `Show message`) (`self.Duration`) true))
  (bind _output_get (set `self.Event Timer Handler` _returnvalue))
  (`KismetSystemLibrary.K2_PauseTimerHandle` _output_get))

(event `Show message`
  (`/Game/Blueprints/Main_BP_SharedFolder/BPF_HUDHelper.ShowToolTip` (`self.Message Text`) (`self.Duration`)))

(event `self.ReceiveActorBeginOverlap`
  (params (OtherActor :type "Actor Object Reference"))
  (cast `MyPlayerCharacter` OtherActor)
  (`KismetSystemLibrary.K2_UnPauseTimerHandle` (`self.Event Timer Handler`)))

(event `self.ReceiveActorEndOverlap`
  (params (OtherActor :type "Actor Object Reference"))
  (cast `MyPlayerCharacter` OtherActor)
  (`KismetSystemLibrary.K2_PauseTimerHandle` (`self.Event Timer Handler`)))

(fn `UserConstructionScript`)