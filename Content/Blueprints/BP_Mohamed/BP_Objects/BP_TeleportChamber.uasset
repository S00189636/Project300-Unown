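; Two-way teleport chamber that moves the player between an entry portal mesh and an exit portal mesh.
; On actor overlap, GetDestination checks which portal the old-v2 player character overlaps and returns the opposite portal's location, where the overlapping actor is teleported.
; Any overlap while ready starts a cooldown, even without a player, and Tick counts it down before re-enabling teleporting.
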(event `self.ReceiveTick`
  (params (DeltaSeconds :type "Float (single-precision)"))
  (if (not (`self.CanTeleport`))
    (bind _output_get (set `self.Timer` (- (`self.Timer`) DeltaSeconds)))
    (if (<= _output_get 0.0)
      (set `self.CanTeleport` true)
      (set `self.Timer` 10.0))))

(event `self.ReceiveActorBeginOverlap`
  (params (OtherActor :type "Actor Object Reference"))
  (if (`self.CanTeleport`)
    (set `self.CanTeleport` false)
    (bind (_isplayer _destination) (`self.Get Destination`))
    (if _isplayer
      (`SceneComponent.K2_SetWorldLocationAndRotation` (`Actor.RootComponent` OtherActor) _destination (`SceneComponent.K2_GetComponentRotation` (`self.parent`)) false true))))

(fn `Get Destination`
  (returns (IsPlayer :type Boolean) (Destination :type "Vector Structure"))
  (bind _sm_portalin (`self.SM_PortalIn`))
  (bind _sm_protalout (`self.SM_protalOut`))
  (bind _returnvalue (> (`KismetArrayLibrary.Array_Length` (`PrimitiveComponent.GetOverlappingActors` _sm_protalout "/Game/Blueprints/Main_BP_SharedFolder/Player/BP_PlayerCharecter_OLD_v2.BP_PlayerCharecter_OLD_v2_C")) 0))
  (bind _returnvalue_2 (> (`KismetArrayLibrary.Array_Length` (`PrimitiveComponent.GetOverlappingActors` _sm_portalin "/Game/Blueprints/Main_BP_SharedFolder/Player/BP_PlayerCharecter_OLD_v2.BP_PlayerCharecter_OLD_v2_C")) 0))
  (if _returnvalue_2
    (return _returnvalue_2 (`SceneComponent.K2_GetComponentLocation` _sm_protalout))
    (elif _returnvalue
      (return _returnvalue (`SceneComponent.K2_GetComponentLocation` _sm_portalin))
      (else
        (return false (0.0 0.0 0.0))))))

(fn `UserConstructionScript`)