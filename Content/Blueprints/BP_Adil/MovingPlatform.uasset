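; MovingPlatform is a Blueprint actor for a platform that moves along a path of three points.
; The construction script fills the InterpToMovement component's control points from three location variables, all relative positions, and sets its duration from a Duration variable.
; The event graph holds no active logic, so movement is left entirely to that component.
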(fn `UserConstructionScript`
  (bind _interptomovement (`self.InterpToMovement`))
  (set `InterpToMovementComponent.ControlPoints` (`|MakeArray` (make `InterpControlPoint` (`self.location1`)) (make `InterpControlPoint` (`self.location2`)) (make `InterpControlPoint` (`self.location3`))) _interptomovement)
  (set `InterpToMovementComponent.Duration` (`self.duration`) _interptomovement))