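; BP_SpinningPlatform2 is a platform actor that spins and pauses at target rotations.
; Each Tick sets the RotatingMovement rate to RotationRate, or to zero while PauseSpin is set.
; When actor rotation nears TurnAmount, it pauses, shrinks TurnAmount to almost zero, and resumes after a DurationBetweenSpins delay.
; An older timer-based spin/pause loop using DurationOfSpin remains unconnected and never runs.
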(event `self.ReceiveBeginPlay`)

(event `self.ReceiveTick`
  (params (DeltaSeconds :type "Float (single-precision)"))
  (if (`self.PauseSpin`)
    (set `RotatingMovementComponent.RotationRate` (struct) (`self.RotatingMovement`))
    (else
      (set `RotatingMovementComponent.RotationRate` (`self.Rotation Rate`) (`self.RotatingMovement`))))
  (if (== (`self.K2_GetActorRotation`) (`self.TurnAmount`) :`ErrorTolerance` 1.0)
    (set `self.PauseSpin` true)
    (set `self.TurnAmount` (* (`self.TurnAmount`) 1e-06))
    (`KismetSystemLibrary.Delay` (`self.durationBetweenSpins`))
    (set `self.PauseSpin` false)))

(fn `UserConstructionScript`)