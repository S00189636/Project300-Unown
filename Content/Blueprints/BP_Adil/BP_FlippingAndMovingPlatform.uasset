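; Moving platform that travels between two points while periodically rotating in short bursts to flip.
; The construction script builds the InterpToMovement path from two relative locations, Location1 and Location2, and applies the Duration variable.
; From BeginPlay, an endless delay loop toggles the RotatingMovement rotation rate, alternating brief spins with longer pauses.
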(event `self.ReceiveBeginPlay`
  (bind _rotatingmovement (`self.RotatingMovement`))
  (`KismetSystemLibrary.Delay` 0.5 :!label _label)
  (set `RotatingMovementComponent.RotationRate` (struct) _rotatingmovement)
  (`KismetSystemLibrary.Delay` 2.0)
  (set `RotatingMovementComponent.RotationRate` (struct :`Yaw` 180.0) _rotatingmovement)
  (goto _label))

(fn `UserConstructionScript`
  (bind _interptomovement (`self.InterpToMovement`))
  (set `InterpToMovementComponent.ControlPoints` (`|MakeArray` (make `InterpControlPoint` (`self.location1`)) (make `InterpControlPoint` (`self.location2`))) _interptomovement)
  (set `InterpToMovementComponent.Duration` (`self.duration`) _interptomovement))