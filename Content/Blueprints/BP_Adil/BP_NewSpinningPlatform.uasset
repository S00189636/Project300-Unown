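; BP_NewSpinningPlatform is a platform that alternates between spinning and standing still, reversing direction with each new spin.
; A looping timer started on BeginPlay calls Spin every DurationOfSpin, where a FlipFlop alternates between setting and zeroing the RotatingMovement rotation rate.
; After each spin rate is applied, the X, Y and Z spin values are negated for the next cycle.
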(event `self.ReceiveBeginPlay`
  (`KismetSystemLibrary.K2_SetTimerDelegate` (delegate `Spin`) (`self.DurationOfSpin`) true))

(event `Spin`
  (`/Engine/EditorBlueprintResources/StandardMacros.FlipFlop`
    (:`A`
      (set `RotatingMovementComponent.RotationRate` (`KismetMathLibrary.MakeRotator` (`self.X_Spin`) (`self.Y_Spin`) (`self.Z_Spin`)) (`self.RotatingMovement`))
      (set `self.Z_Spin` (* -1 (`self.Z_Spin`)))
      (set `self.X_Spin` (* -1 (`self.X_Spin`)))
      (set `self.Y_Spin` (* -1 (`self.Y_Spin`))))
    (:`B`
      (set `RotatingMovementComponent.RotationRate` (struct) (`self.RotatingMovement`)))))

(fn `UserConstructionScript`)