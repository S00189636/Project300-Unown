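; Two-way portal actor that teleports overlapping actors between its two portal meshes and plays a sound.
; Tick moves both portal view components to the player camera's position mirrored through the portals' midpoint, copying the camera's rotation.
; On overlap, GetDestination checks which mesh has overlapping actors and returns the other's location and forward rotation.
; CanTeleport guards re-entry but only resets after a successful teleport.
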(event `self.ReceiveTick`
  (params (DeltaSeconds :type "Float (single-precision)"))
  (bind _transformcomponent (`PlayerCameraManager.TransformComponent` (`PlayerController.PlayerCameraManager` (`GameplayStatics.GetPlayerController` 0))))
  (bind _transformcomponent_2 (`PlayerCameraManager.TransformComponent` (`PlayerController.PlayerCameraManager` (`GameplayStatics.GetPlayerController` 0))))
  (`SceneComponent.K2_SetWorldLocationAndRotation` (`self.OutPortalView1`) (- (+ (`SceneComponent.K2_GetComponentLocation` (`self.SM_PortalIn`)) (`SceneComponent.K2_GetComponentLocation` (`self.SM_protalOut`))) (`SceneComponent.K2_GetComponentLocation` _transformcomponent_2)) (`SceneComponent.K2_GetComponentRotation` _transformcomponent_2) false false)
  (`SceneComponent.K2_SetWorldLocationAndRotation` (`self.InPortalView`) (- (+ (`SceneComponent.K2_GetComponentLocation` (`self.SM_PortalIn`)) (`SceneComponent.K2_GetComponentLocation` (`self.SM_protalOut`))) (`SceneComponent.K2_GetComponentLocation` _transformcomponent)) (`SceneComponent.K2_GetComponentRotation` _transformcomponent) false false))

(event `self.ReceiveActorBeginOverlap`
  (params (OtherActor :type "Actor Object Reference"))
  (if (`self.CanTeleport`)
    (set `self.CanTeleport` false)
    (bind (_isplayer _destination _rotation) (`self.Get Destination`))
    (if _isplayer
      (`SceneComponent.K2_SetWorldLocationAndRotation` (`Actor.RootComponent` OtherActor) _destination _rotation false false)
      (set `self.CanTeleport` true)
      (`GameplayStatics.PlaySound2D` "/Game/Sounds/SE_Simran/Teleport_Committed.Teleport_Committed" 0.5 1.0 0.0 null null))))

(fn `Get Destination`
  (returns (IsPlayer :type Boolean) (Destination :type "Vector Structure") (Rotation :type "Rotator Structure"))
  (bind _sm_portalin (`self.SM_PortalIn`))
  (bind _sm_protalout (`self.SM_protalOut`))
  (bind _returnvalue (> (`KismetArrayLibrary.Array_Length` (`PrimitiveComponent.GetOverlappingActors` _sm_protalout null)) 0))
  (bind _returnvalue_2 (> (`KismetArrayLibrary.Array_Length` (`PrimitiveComponent.GetOverlappingActors` _sm_portalin "/Script/Engine.Actor")) 0))
  (if _returnvalue_2
    (return _returnvalue_2 (`SceneComponent.K2_GetComponentLocation` _sm_protalout) (`KismetMathLibrary.Conv_VectorToRotator` (`SceneComponent.GetForwardVector` _sm_protalout)))
    (elif _returnvalue
      (return _returnvalue (`SceneComponent.K2_GetComponentLocation` _sm_portalin) (`KismetMathLibrary.Conv_VectorToRotator` (`SceneComponent.GetForwardVector` _sm_portalin))))))

(fn `UserConstructionScript`)