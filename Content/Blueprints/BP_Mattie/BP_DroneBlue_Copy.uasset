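; BP_DroneBlue_Copy is an enemy drone that hunts and shoots at the player character.
; Pawn sensing locks the first seen player as Target and plays a sound.
; Tick moves the drone toward the target until within attack range, then strafes sideways while firing projectiles on a short cooldown, smoothing rotation with a lerp.
; A self-restarting, randomly timed timer uses a FlipFlop to alternate strafe direction.
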(event `ChangeStrafe`
  (bind _isa (`/Engine/EditorBlueprintResources/StandardMacros.FlipFlop`)
    (:`A`
      _)
    (:`B`
      _))
  (set `self.StrafeRight` _isa)
  (`KismetSystemLibrary.K2_SetTimerDelegate` (delegate `ChangeStrafe`) (`KismetMathLibrary.RandomFloatInRange` 2.0 5.0)))

(event `self.ReceiveBeginPlay`
  (`self.ChangeStrafe`))

(event `self.ReceiveTick`
  (params (DeltaSeconds :type "Float (single-precision)"))
  (bind _target (`self.Target`)
    (:`then`
      (if (> (`self.GetDistanceTo` _target) (`self.AttackRange`))
        (bind _returnvalue (+ (`self.K2_GetActorLocation` _target) (0.0 0.0 100.0)))
        (bind (_returnvalue_roll _returnvalue_pitch _returnvalue_yaw) (`KismetMathLibrary.BreakRotator` (`KismetMathLibrary.FindLookAtRotation` (`self.K2_GetActorLocation`) _returnvalue)))
        (`self.AddMovementInput` (`KismetMathLibrary.Conv_RotatorToVector` (`KismetMathLibrary.MakeRotator` 0.0 0.0 _returnvalue_yaw)))
        (`self.K2_SetActorRotation` (`KismetMathLibrary.RLerp` (`self.K2_GetActorRotation`) (`KismetMathLibrary.MakeRotator` 0.0 0.0 _returnvalue_yaw) 0.1 true))
        (else
          (bind _returnvalue_2 (`KismetMathLibrary.FindLookAtRotation` (`self.K2_GetActorLocation`) _returnvalue))
          (`self.AddMovementInput` (`KismetMathLibrary.GetRightVector` _returnvalue_2) (`KismetMathLibrary.SelectFloat` 1.0 -1.0 (`self.StrafeRight`)))
          (`self.K2_SetActorRotation` (`KismetMathLibrary.RLerp` (`self.K2_GetActorRotation`) _returnvalue_2 0.1 true))
          (if (`self.CanAttack`)
            (set `self.CanAttack` false)
            (`self.FireProjectile`)
            (`KismetSystemLibrary.Delay` 0.5)
            (set `self.CanAttack` true)))))
    (:`else`)))

(event `self.PawnSensing.OnSeePawn`
  (params (Pawn :type "Pawn Object Reference"))
  (bind _asbp_mattie_player_character (cast `/Game/Blueprints/BP_Mattie/Mattie/Blueprints/BP_Mattie_PlayerCharacter` Pawn))
  (`self.Target`
    (:`then`)
    (:`else`
      (set `self.Target` _asbp_mattie_player_character)
      (`GameplayStatics.PlaySound2D` "/Engine/VREditor/Sounds/VR_open.VR_open" 1.0 1.0 0.0 null null))))

(event `FireProjectile`
  (`|SpawnActorFromClass` "/Game/Blueprints/BP_Simran/BP_Projectile.BP_Projectile_C" (`SceneComponent.K2_GetComponentToWorld` (`self.ProjectileSpawn`)) "AlwaysSpawn" "OverrideRootScale" null 0.0 null))

(fn `UserConstructionScript`)