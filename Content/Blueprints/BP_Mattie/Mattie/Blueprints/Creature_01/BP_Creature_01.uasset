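; Creature blueprint that damages the player and can leave a trail of ground stamps.
; Attack applies damage through the player's MainPlayerState, gated by a delay-based cooldown.
; A looping fast timer, paused until StartStopStampEvent resumes it, spawns unattached static mesh components at the capsule's location.
; ToggleInvisibility swaps the mesh between AttackMaterial and a saved default through dynamic instances, and Die switches it to AttackMaterial.
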(event `self.ReceiveBeginPlay`
  (`parent.ReceiveBeginPlay`)
  (bind _returnvalue (`KismetSystemLibrary.K2_SetTimerDelegate` (delegate `AIGroundStamp`) 0.01 true))
  (bind _output_get (set `self.StampTimeHandler` _returnvalue))
  (`KismetSystemLibrary.K2_PauseTimerHandle` _output_get))

(event `AIGroundStamp`
  (`/Engine/EditorBlueprintResources/StandardMacros.IsValid` (`self.CapsuleComponent`)
    (:`Is Valid`
      (`AddComponent|NODE_AddStaticMeshComponent-0` :`bManualAttachment` true :`RelativeTransform` (`KismetMathLibrary.Conv_VectorToTransform` (`SceneComponent.K2_GetComponentLocation` (`self.CapsuleComponent`)))))))

(event `self.Attack`
  (params (TargetActor :type "Actor Object Reference"))
  (if (`self.RedyToAttack`)
    (bind _asmain_player_state (cast `MainPlayerState` (`Pawn.PlayerState` (`GameplayStatics.GetPlayerCharacter` 0))))
    (`MainPlayerState.TakeDamageToHealth` _asmain_player_state (`self.DamageAmount`))
    (set `self.RedyToAttack` false)
    (`KismetSystemLibrary.Delay` (`self.AttackRate`))
    (set `self.RedyToAttack` true)))

(fn `Die`
  (`parent.Die`)
  (`self.ToggleInvisibility` true))

(fn `StartStopStampEvent`
  (params (IsStamping :type Boolean))
  (if IsStamping
    (`KismetSystemLibrary.K2_UnPauseTimerHandle` (`self.StampTimeHandler`))
    (else
      (`KismetSystemLibrary.K2_PauseTimerHandle` (`self.StampTimeHandler`)))))

(fn `ToggleInvisibility`
  (params (Condition :type Boolean))
  (bind _mesh (`self.Mesh`))
  (if Condition
    (bind _returnvalue (`PrimitiveComponent.CreateDynamicMaterialInstance` _mesh 0 (`|GetArrayItem` (`MeshComponent.GetMaterials` _mesh)) "None"))
    (set `self.DefaultMaterial` _returnvalue)
    (`PrimitiveComponent.CreateDynamicMaterialInstance` (`self.Mesh`) 0 (`self.AttackMaterial`) "None")
    (else
      (`PrimitiveComponent.CreateDynamicMaterialInstance` (`self.Mesh`) 0 (`self.DefaultMaterial`) "None"))))

(fn `UserConstructionScript`
  (`parent.UserConstructionScript`))