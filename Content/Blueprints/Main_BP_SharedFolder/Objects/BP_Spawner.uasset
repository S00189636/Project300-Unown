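; BP_Spawner is a placeable spawner that creates a limited number of actors of a configurable class at its own transform.
; A looping timer spawns one actor per interval and pauses once the spawn count is reached.
; The timer runs from BeginPlay when StartOnBeginPlay is set; otherwise it stays paused until MyPlayerCharacter overlaps the Box trigger.
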(event `self.ReceiveBeginPlay`
  (bind _returnvalue (`KismetSystemLibrary.K2_SetTimerDelegate` (delegate `Spawn`) (`self.TimeToSpawn`) true))
  (bind _output_get (set `self.SpawnTimerHandler` _returnvalue))
  (if (`self.StartOnBeginPlay`)
    (set `self.Triggered` true)
    (else
      (`KismetSystemLibrary.K2_PauseTimerHandle` _output_get))))

(event `Spawn`
  (if (< (`self.CurrentCount`) (`self.SpawnCount`))
    (`|SpawnActorFromClass` (`self.ActorClassToSpawn`) (`self.GetTransform`) "AdjustIfPossibleButAlwaysSpawn" "OverrideRootScale" null null)
    (`/Engine/EditorBlueprintResources/StandardMacros.IncrementInt` (`self.CurrentCount`))
    (else
      (`KismetSystemLibrary.K2_PauseTimerHandle` (`self.SpawnTimerHandler`)))))

(event `self.Box.OnComponentBeginOverlap`
  (params (OverlappedComponent :type "PrimitiveComponent Object Reference") (OtherActor :type "Actor Object Reference") (OtherComp :type "PrimitiveComponent Object Reference") (OtherBodyIndex :type Integer) (bFromSweep :type Boolean) (SweepResult :type "HitResult Structure (by ref)"))
  (if (not (`self.Triggered`))
    (cast `MyPlayerCharacter` OtherActor)
    (`KismetSystemLibrary.K2_UnPauseTimerHandle` (`self.SpawnTimerHandler`))))

(fn `UserConstructionScript`)