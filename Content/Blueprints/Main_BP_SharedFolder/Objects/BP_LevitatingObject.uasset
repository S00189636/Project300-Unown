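; Levitatable object that glows while levitated and damages BI_Damageable actors its mesh hits.
; StartLevitate turns the aura on and returns the StaticMesh to the caller, leaving Power and Direction unused; EndLevitate turns it off.
; ToggleAura caches the current material, swaps in a dynamic M_FloatingGlow_Inst, and restores the cached one afterwards.
; Hit damage scales with the mesh's bounding-sphere radius, whether levitating or not.
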(event `self.StaticMesh.OnComponentHit`
  (params (HitComponent :type "PrimitiveComponent Object Reference") (OtherActor :type "Actor Object Reference") (OtherComp :type "PrimitiveComponent Object Reference") (NormalImpulse :type "Vector Structure") (Hit :type "HitResult Structure (by ref)"))
  (if (`KismetSystemLibrary.DoesImplementInterface` OtherActor "/Game/Blueprints/BP_Mohamed/BI_Damageable.BI_Damageable_C")
    (message `/Game/Blueprints/BP_Mohamed/BI_Damageable.TakeDamage` OtherActor "NewEnumerator1" (* (`.SphereRadius` (`KismetSystemLibrary.GetComponentBounds` HitComponent)) 0.1))))

(fn `EndLevitate`
  (returns (Ended :type Boolean))
  (`self.ToggleAura` 0)
  (return false))

(fn `StartLevitate`
  (params (Power :type "Float (double-precision)") (Direction :type "Vector Structure"))
  (returns (outComp :type "PrimitiveComponent Object Reference"))
  (`self.ToggleAura` 1)
  (return (`self.StaticMesh`)))

(fn `ToggleAura`
  (params (isOn :type Integer))
  (bind _staticmesh (`self.StaticMesh`))
  (if (> isOn 0)
    (bind _returnvalue (`PrimitiveComponent.CreateDynamicMaterialInstance` _staticmesh 0 (`|GetArrayItem` (`MeshComponent.GetMaterials` _staticmesh)) "None"))
    (set `self.DefaultMaterial` _returnvalue)
    (bind _returnvalue_2 (`PrimitiveComponent.CreateDynamicMaterialInstance` _staticmesh 0 "/Game/Materials/M_Mohamed/M_FloatingGlow_Inst.M_FloatingGlow_Inst" "None"))
    (`MaterialInstanceDynamic.SetScalarParameterValue` _returnvalue_2 "IsAuraOn" (`KismetMathLibrary.Conv_IntToDouble` 1))
    (else
      (`PrimitiveComponent.CreateDynamicMaterialInstance` (`self.StaticMesh`) 0 (`self.DefaultMaterial`) "None"))))

(fn `UserConstructionScript`)