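; BP_Game is the Game Instance that centralizes level travel, input mode and UI flow for the game.
; It lazily creates and reuses the HUD, pause and game-over widgets, switching pause and cursor state with them.
; Lab terminal selection stores a level, picks its loading-screen background and ends selection, while a separate event opens that level.
; It also holds health and mana values for the HUD, normalized from amount and maximum.
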(event `OpenLevel`
  (params (LevelName :type Name))
  (`GameplayStatics.OpenLevel` LevelName)
  (`self.ShowPlayerHUD`)
  (`self.SetInputMode` false))

(event `GoToSelectedLevel`
  (`GameplayStatics.OpenLevel` (`self.SelectedLevel`)))

(event `SelectLevel`
  (params (SelectedLevel :type Name))
  ;[1 1 1] Set Loading Screen For Selected Level (Lab Terminal)
  (bind _output_get (set `self.SelectedLevel` SelectedLevel))
  (if (== _output_get "Level1")
    (`self.SetLoadingScreenIndex` 0)
    (elif (== (`self.SelectedLevel`) "Level2")
      (`self.SetLoadingScreenIndex` 1)
      (elif (== (`self.SelectedLevel`) "Level3")
        (`self.SetLoadingScreenIndex` 2)
        (elif (== (`self.SelectedLevel`) "Level4")
          (`self.SetLoadingScreenIndex` 3))))))

(event `SetInputMode`
  (params (`IsUI?` :type Boolean))
  (bind _returnvalue (`GameplayStatics.GetPlayerController` 0))
  (bind _returnvalue_2 (`GameplayStatics.GetPlayerController` 0))
  (if `IsUI?`
    (`WidgetBlueprintLibrary.SetInputMode_UIOnlyEx` _returnvalue null)
    (set `PlayerController.bShowMouseCursor` true _returnvalue)
    (else
      (`WidgetBlueprintLibrary.SetInputMode_GameOnly` _returnvalue_2)
      (set `PlayerController.bShowMouseCursor` false _returnvalue_2))))

(event `ShowPlayerHUD`
  ;[1 1 1] Show Player HUD
  (`/Engine/EditorBlueprintResources/StandardMacros.IsValid` (`self.PlayerHUD`)
    (:`Is Valid`
      (`Widget.SetVisibility` (`self.PlayerHUD`) "Visible"))
    (:`Is Not Valid`
      (bind _returnvalue (`|CreateWidget` "/Game/Blueprints/BP_Mattie/HUD/UMG_MainHUD.UMG_MainHUD_C" (`GameplayStatics.GetPlayerController` 0)))
      (set `self.PlayerHUD` _returnvalue)))
  (if (not (`Widget.IsInViewport` (`self.PlayerHUD`)))
    (`UserWidget.AddToViewport` (`self.PlayerHUD`) 0)
    (bind _asmain_player_state (cast `MainPlayerState` (`Pawn.PlayerState` (`GameplayStatics.GetPlayerCharacter` 0))))
    (set `self.ManaToHUD` (`MainPlayerState.CurrentMana` _asmain_player_state))
    (set `self.HealthToHUD` (`MainPlayerState.CurrentHealth` _asmain_player_state))))

(event `EndLevelSelect`
  (bind _returnvalue (`GameplayStatics.GetActorOfClass` "/Game/Blueprints/BP_Mohamed/BP_LevelSelectTerminal.BP_LevelSelectTerminal_C"))
  (`/Engine/EditorBlueprintResources/StandardMacros.IsValid` _returnvalue
    (:`Is Valid`
      (`/Game/Blueprints/BP_Mohamed/BP_LevelSelectTerminal.EndSelection` _returnvalue)
      (`self.ShowPlayerHUD`))))

(event `HidePlayerHUD`
  ;[1 1 1] Hide Player HUD
  (`/Engine/EditorBlueprintResources/StandardMacros.IsValid` (`self.PlayerHUD`)
    (:`Is Valid`
      (`Widget.SetVisibility` (`self.PlayerHUD`) "Hidden"))))

(event `Resume`
  (`self.ShowPlayerHUD`)
  (`self.SetInputMode` false)
  (`GameplayStatics.SetGamePaused` false)
  (`Widget.SetVisibility` (`self.PauseMenu`) "Hidden"))

(event `Pause`
  (`self.HidePlayerHUD`)
  (`self.SetInputMode` true)
  (`GameplayStatics.SetGamePaused` true)
  (`/Engine/EditorBlueprintResources/StandardMacros.IsValid` (`self.PauseMenu`)
    (:`Is Valid`
      _)
    (:`Is Not Valid`
      (bind _returnvalue (`|CreateWidget` "/Game/Blueprints/BP_Mohamed/UI/UMG_PauseMenu.UMG_PauseMenu_C" (`GameplayStatics.GetPlayerController` 0)))
      (set `self.PauseMenu` _returnvalue)))
  (if (`Widget.IsInViewport` (`self.PauseMenu`))
    (`Widget.SetVisibility` (`self.PauseMenu`) "Visible")
    (else
      (`Widget.SetVisibility` (`self.PauseMenu`) "Visible")
      (`UserWidget.AddToViewport` (`self.PauseMenu`) 0))))

(event `self.Die`
  (`self.SetInputMode` true)
  (`GameplayStatics.SetGamePaused` true)
  (`/Engine/EditorBlueprintResources/StandardMacros.IsValid` (`self.GameOver`)
    (:`Is Valid`
      _)
    (:`Is Not Valid`
      (bind _returnvalue (`|CreateWidget` "/Game/Materials/M_Simran/UMG_GameOver.UMG_GameOver_C" (`GameplayStatics.GetPlayerController` 0)))
      (set `self.GameOver` _returnvalue)))
  (if (`Widget.IsInViewport` (`self.GameOver`))
    (`Widget.SetVisibility` (`self.GameOver`) "Visible")
    (else
      (`UserWidget.AddToViewport` (`self.GameOver`) 0))))

(event `self.SetHealthHUDValueFromAmount`
  (params (amount :type "Float (single-precision)") (maxAmount :type "Float (single-precision)"))
  (set `self.HealthToHUD` (`KismetMathLibrary.NormalizeToRange` (/ amount maxAmount) 0.0 1.0)))

(event `self.SetManaHUDValueFromAmount`
  (params (amount :type "Float (single-precision)") (maxAmount :type "Float (single-precision)"))
  (set `self.ManaToHUD` (`KismetMathLibrary.NormalizeToRange` (/ amount maxAmount) 0.0 1.0)))

(fn `SetLoadingScreenIndex`
  (params (BackgroundIndex :type Integer))
  (`AsyncLoadingScreenLibrary.SetDisplayBackgroundIndex` BackgroundIndex)
  (bind _asbp_game (cast `/Game/Blueprints/Main_BP_SharedFolder/BP_Game` (`GameplayStatics.GetGameInstance`)))
  (`self.EndLevelSelect` _asbp_game)
  (`self.SetInputMode` false))