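; Base enemy Blueprint with health, typed damage, death and hooks for being levitated.
; TakeDamage filters hits by the accepted damage type, then calls SubtractHealth and Die, which switches state, ragdolls the mesh and destroys the capsule.
; StartLevitate applies power as damage and hands back the mesh when that reports death; EndLevitate restores gravity.
; Attack is a cooldown-gated placeholder that only prints, alongside a LookAtActor rotation helper.
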(event `self.ReceiveBeginPlay`
  (`parent.ReceiveBeginPlay`)
  (set `self.ReturnComp` (`self.Mesh`))
  (`self.SubtractHealth` (* -1 (`self.MaxHealth`))))

(event `Attack`
  (params (TargetActor :type "Actor Object Reference"))
  (if (`self.RedyToAttack`)
    (`KismetSystemLibrary.PrintString` "Enemy Attacking")
    (set `self.RedyToAttack` false)
    (`KismetSystemLibrary.Delay` (`self.AttackRate`))
    (set `self.RedyToAttack` true)))

(fn `Die`
  (bind _capsulecomponent (`self.CapsuleComponent`))
  (if (not (`|EnumEquality` (`self.State`) "NewEnumerator5"))
    (`self.SetState` "NewEnumerator5")
    (`PrimitiveComponent.SetSimulatePhysics` (`self.ReturnComp`) true)
    (if (`KismetSystemLibrary.IsValid` _capsulecomponent)
      (`ActorComponent.K2_DestroyComponent` _capsulecomponent))
    (`PrimitiveComponent.SetCollisionResponseToChannel` (`self.ReturnComp`) "ECC_Visibility" "ECR_Block")))

(fn `EndLevitate`
  (returns (Ended :type Boolean))
  (`PrimitiveComponent.SetEnableGravity` (`self.Mesh`) true)
  (return false))

(fn `LookAtActor`
  (params (OtherActor :type "Actor Object Reference"))
  (`self.K2_SetActorRotation` (`KismetMathLibrary.MakeRotator` (.roll (`KismetMathLibrary.FindLookAtRotation` (`self.K2_GetActorLocation`) (`self.K2_GetActorLocation` OtherActor))) 0.0 (.yaw (`KismetMathLibrary.FindLookAtRotation` (`self.K2_GetActorLocation`) (`self.K2_GetActorLocation` OtherActor))))))

(fn `SetState`
  (params (State :type "/Game/Blueprints/Main_BP_SharedFolder/AI/E_EnemyState Enum" :default "NewEnumerator0"))
  (set `self.PreviousState` (`self.State`))
  (set `self.State` State))

(fn `StartLevitate`
  (params (Power :type "Float (double-precision)") (Direction :type "Vector Structure"))
  (returns (outComp :type "PrimitiveComponent Object Reference"))
  (`self.SetState` "NewEnumerator4")
  (bind _dead (`self.TakeDamage` "NewEnumerator0" Power))
  (if _dead
    (return (`self.ReturnComp`))))

(fn `TakeDamage`
  (params (DamageType :type "/Game/Blueprints/BP_Mohamed/E_DamageType Enum" :default "NewEnumerator0") (Amount :type "Float (double-precision)"))
  (returns (Dead :type Boolean))
  ;[1 1 1] If Dead Don't do anything
  (if (`|EnumInequality` (`self.State`) "NewEnumerator5")
    ;[1 1 1] Check Damage Type
    (if (`|EnumEquality` (`self.TakeDamageFromType`) "NewEnumerator3")
      _
      (elif (`|EnumEquality` DamageType (`self.TakeDamageFromType`))
        _
        (else
          (`KismetSystemLibrary.PrintString` "This dose not work on me ")
          (return false))))
    ;[1 1 1] If Health is at 0 call die function
    (bind _returnvalue (`self.SubtractHealth` Amount))
    (if _returnvalue
      (`self.Die`)
      (return true)
      (else
        (return false)))
    (else
      (return true))))

(fn `UserConstructionScript`)