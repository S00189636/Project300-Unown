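; BPF_HUDHelper is a Blueprint function library of shortcuts for HUD-related game access.
; ShowToolTip casts the game instance to BP_Game and forwards tooltip text and duration to it.
; The two getters return the first local player's MainPlayerState and MyPlayerCharacter through player index 0, proceeding only when the cast succeeds.
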(fn `GetMyPlayerCharacter`
  (returns (`AsMy Player Character` :type "MyPlayerCharacter Object Reference"))
  (bind _asmy_player_character (cast `MyPlayerCharacter` (`GameplayStatics.GetPlayerCharacter` (`local.__WorldContext`))))
  (return _asmy_player_character))

(fn `GetMyPlayerState`
  (returns (`AsMain Player State` :type "MainPlayerState Object Reference"))
  (bind _asmain_player_state (cast `MainPlayerState` (`Controller.PlayerState` (`GameplayStatics.GetPlayerController` (`local.__WorldContext`)))))
  (return _asmain_player_state))

(fn `ShowToolTip`
  (params (ToolTipText :type String) (Duration :type "Float (double-precision)"))
  (bind _asbp_game (cast `/Game/Blueprints/Main_BP_SharedFolder/BP_Game` (`GameplayStatics.GetGameInstance` (`local.__WorldContext`))))
  (`/Game/Blueprints/Main_BP_SharedFolder/BP_Game.ShowToolTip` _asbp_game ToolTipText Duration))